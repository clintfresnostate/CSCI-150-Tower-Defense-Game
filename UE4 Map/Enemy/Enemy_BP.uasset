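; Enemy actor that follows the first valid Path actor's spline and has separate red, green and blue health pools.
; AnyDamage drains the pool matching the damage type, shows floating text, and explodes and destroys the enemy once all three are empty.
; A dynamic material on the sphere reflects each pool's damage through scalar parameters.
; Tick refreshes the health widget's bars and advances a fixed distance along the spline, making speed frame-rate dependent.
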(event EventTick
  (params (DeltaSeconds :type Float%20%28single-precision%29))
  (bind _asenemy_health (Utilities|Casting|CastToEnemy_Health (UserInterface|GetUserWidgetObject (Variables|Default|GetWidget))))
  (Progress|SetPercent (Variables|/Game/UI/Enemy_Health.Enemy_Health_C|GetBlue _asenemy_health) (/ (Variables|Default|GetBlue_Health) 1e+03))
  (Progress|SetPercent (Variables|/Game/UI/Enemy_Health.Enemy_Health_C|Getred _asenemy_health) (/ (Variables|Default|GetRed_Health) 1e+03))
  (Progress|SetPercent (Variables|/Game/UI/Enemy_Health.Enemy_Health_C|Getgreen _asenemy_health) (/ (Variables|Default|GetGreen_Health) 1e+03))
  (CallFunction|UpdatePathing))

(event EventBeginPlay
  (bind _dynamicmat (Variables|Default|GetDynamicMat))
  (Rendering|Material|SetScalarParameterValue _dynamicmat "Green Damage" (- 1.0 (/ (Variables|Default|GetGreen_Health) 1e+03)) :!class /Script/Engine.MaterialInstanceDynamic)
  (Rendering|Material|SetScalarParameterValue _dynamicmat "Red Damage" (- 1.0 (/ (Variables|Default|GetRed_Health) 1e+03)) :!class /Script/Engine.MaterialInstanceDynamic)
  (Rendering|Material|SetScalarParameterValue _dynamicmat "Blue Damage" (- 1.0 (/ (Variables|Default|GetBlue_Health) 1e+03)) :!class /Script/Engine.MaterialInstanceDynamic)
  (bind _outactors (Actor|GetAllActorsOfClass "/Game/SplinePathway/Path.Path_C"))
  (bind _array_element (Utilities|Array|ForEachLoopwithBreak _outactors :!label _label)
    (:LoopBody
      (if (Utilities|IsValid _array_element)
        (Variables|Default|SetSplineRef _array_element)
        (Variables|Default|SetDistanceAlongPath 0.0)
        (goto _label Break)))))

(event Game|Damage|EventAnyDamage
  (params (Damage :type Float%20%28single-precision%29) (DamageType :type Damage%20Type%20Object%20Reference) (InstigatedBy :type Controller%20Object%20Reference) (DamageCauser :type Actor%20Object%20Reference))
  (bind _dynamicmat (Variables|Default|GetDynamicMat))
  (bind _returnvalue (UserInterface|CreateWidget "/Game/UI/Floating_Text.Floating_Text_C" 0 self))
  (Variables|/Game/UI/Floating_Text.Floating_Text_C|SetFloatText _returnvalue Damage)
  (UserInterface|Viewport|AddtoViewport _returnvalue 0)
  (UserInterface|Animation|PlayAnimation _returnvalue (Variables|/Game/UI/Floating_Text.Floating_Text_C|GetFloating%20Text%20Animation _returnvalue) 0.0 1 "Forward")
  (bind _asred_damage (Utilities|Casting|CastToRedDamage DamageType)
    (:then
      _)
    (:CastFailed
      _))
  (bind _asgreen_damage (Utilities|Casting|CastToGreenDamage DamageType)
    (:then
      _)
    (:CastFailed
      _))
  (bind _asblue_damage (Utilities|Casting|CastToBlueDamage DamageType)
    (:then
      _)
    (:CastFailed
      _))
  (Variables|Default|SetDamage Damage)
  (if (== DamageType _asblue_damage)
    (bind _returnvalue_2 (Rendering|Material|GetScalarParameterValue _dynamicmat "Blue Damage" :!class /Script/Engine.MaterialInstanceDynamic))
    (Variables|/Game/UI/Floating_Text.Floating_Text_C|SetBlueDamage _returnvalue _returnvalue_2)
    (Rendering|Material|SetScalarParameterValue _dynamicmat "Blue Damage" (+ _returnvalue_2 (/ (Variables|Default|GetDamage) 1e+03)) :!class /Script/Engine.MaterialInstanceDynamic)
    (Variables|Default|SetBlue_Health (- (Variables|Default|GetBlue_Health) (Variables|Default|GetDamage)))
    (bind _health_0 (CallFunction|CheckHealth<=0 :!label _label))
    (if _health_0
      (Effects|SpawnEmitteratLocation "/Game/StarterContent/Particles/P_Explosion.P_Explosion" (Transformation|GetActorLocation))
      (Rendering|SetActorHiddenInGame true)
      (Utilities|FlowControl|Delay 0.2)
      (Actor|DestroyActor))
    (elif (== DamageType _asred_damage)
      (bind _returnvalue_3 (Rendering|Material|GetScalarParameterValue _dynamicmat "Red Damage" :!class /Script/Engine.MaterialInstanceDynamic))
      (Variables|/Game/UI/Floating_Text.Floating_Text_C|SetRedDamage _returnvalue _returnvalue_3)
      (Rendering|Material|SetScalarParameterValue _dynamicmat "Red Damage" (+ _returnvalue_3 (/ (Variables|Default|GetDamage) 1e+03)) :!class /Script/Engine.MaterialInstanceDynamic)
      (Variables|Default|SetRed_Health (- (Variables|Default|GetRed_Health) (Variables|Default|GetDamage)))
      (goto _label)
      (elif (== DamageType _asgreen_damage)
        (bind _returnvalue_4 (Rendering|Material|GetScalarParameterValue _dynamicmat "Green Damage" :!class /Script/Engine.MaterialInstanceDynamic))
        (Variables|/Game/UI/Floating_Text.Floating_Text_C|SetGreenDamage _returnvalue _returnvalue_4)
        (Rendering|Material|SetScalarParameterValue _dynamicmat "Green Damage" (+ _returnvalue_4 (/ (Variables|Default|GetDamage) 1e+03)) :!class /Script/Engine.MaterialInstanceDynamic)
        (Variables|Default|SetGreen_Health (- (Variables|Default|GetGreen_Health) (Variables|Default|GetDamage)))
        (goto _label)))))

(fn ConstructionScript
  (bind _returnvalue (Rendering|Material|CreateDynamicMaterialInstance (Variables|Default|GetSphere) 0 "/Game/Enemy/Mat/Enemy_Mat.Enemy_Mat" :!class /Script/Engine.PrimitiveComponent))
  (Variables|Default|SetDynamicMat _returnvalue))

(fn CheckHealth<=0
  (if (Math|Boolean|ANDBoolean (<= (Variables|Default|GetBlue_Health) 0.0) (<= (Variables|Default|GetRed_Health) 0.0) (<= (Variables|Default|GetGreen_Health) 0.0))
    (Variables|Default|SetReturn_Death true)
    (else
      (Variables|Default|SetReturn_Death false)))
  (return (Variables|Default|GetReturn_Death)))

(fn UpdatePathing
  (Transformation|SetActorLocation (Class|SplineComponent|GetWorldLocationatDistanceAlongSpline (Variables|/Game/SplinePathway/Path.Path_C|GetSpline (Variables|Default|GetSplineRef)) (Variables|Default|GetDistanceAlongPath)) false false)
  (Variables|Default|SetDistanceAlongPath (+ (Variables|Default|GetDistanceAlongPath) 2.0)))