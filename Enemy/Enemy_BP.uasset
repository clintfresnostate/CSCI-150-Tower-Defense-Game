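; Enemy Blueprint that records red, green and blue damage taken on its sphere's material.
; The construction script creates a dynamic instance of Enemy_Mat on the Sphere.
; AnyDamage uses casts to identify the damage type and adds the amount to the matching scalar parameter, so the material itself holds each running total.
; No health or death logic is present.
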(event Game|Damage|EventAnyDamage
  (params (Damage :type Float%20%28single-precision%29) (DamageType :type Damage%20Type%20Object%20Reference) (InstigatedBy :type Controller%20Object%20Reference) (DamageCauser :type Actor%20Object%20Reference))
  (bind _dynamicmat (Variables|Default|GetDynamicMat))
  (bind _asred_damage (Utilities|Casting|CastToRedDamage DamageType)
    (:then
      _)
    (:CastFailed
      _))
  (bind _asgreen_damage (Utilities|Casting|CastToGreenDamage DamageType)
    (:then
      _)
    (:CastFailed
      _))
  (bind _asblue_damage (Utilities|Casting|CastToBlueDamage DamageType)
    (:then
      _)
    (:CastFailed
      _))
  (Variables|Default|SetDamage Damage)
  (if (== DamageType _asblue_damage)
    (bind _returnvalue (Rendering|Material|GetScalarParameterValue _dynamicmat "Blue Damage" :!class /Script/Engine.MaterialInstanceDynamic))
    (Rendering|Material|SetScalarParameterValue _dynamicmat "Blue Damage" (+ _returnvalue (Variables|Default|GetDamage)) :!class /Script/Engine.MaterialInstanceDynamic)
    (elif (== DamageType _asred_damage)
      (bind _returnvalue_2 (Rendering|Material|GetScalarParameterValue _dynamicmat "Red Damage" :!class /Script/Engine.MaterialInstanceDynamic))
      (Rendering|Material|SetScalarParameterValue _dynamicmat "Red Damage" (+ _returnvalue_2 (Variables|Default|GetDamage)) :!class /Script/Engine.MaterialInstanceDynamic)
      (elif (== DamageType _asgreen_damage)
        (bind _returnvalue_3 (Rendering|Material|GetScalarParameterValue _dynamicmat "Green Damage" :!class /Script/Engine.MaterialInstanceDynamic))
        (Rendering|Material|SetScalarParameterValue _dynamicmat "Green Damage" (+ _returnvalue_3 (Variables|Default|GetDamage)) :!class /Script/Engine.MaterialInstanceDynamic)))))

(event EventBeginPlay)

(fn ConstructionScript
  (bind _returnvalue (Rendering|Material|CreateDynamicMaterialInstance (Variables|Default|GetSphere) 0 "/Game/Enemy/Enemy_Mat.Enemy_Mat" :!class /Script/Engine.PrimitiveComponent))
  (Variables|Default|SetDynamicMat _returnvalue))