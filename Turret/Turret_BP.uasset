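; Turret actor that attacks Enemy_BP actors in range with red, blue and green typed damage.
; A range sphere fills an enemy array, from which it picks the first enemy with health in a color it damages.
; Tick checks range, fires on cooldown and retargets a lightning beam tinted by the damage mix between shots.
; R and F keys move the turret to fixed offsets; the projectile path is unconnected.
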(event OnComponentBeginOverlap(Range)
  (params (OtherActor :type Actor%20Object%20Reference) (OtherComp :type Primitive%20Component%20Object%20Reference) (OtherBodyIndex :type Integer) (bFromSweep :type Boolean) (SweepResult :type Hit%20Result%20Structure%20%28by%20ref%29))
  (Utilities|Array|Add (Variables|Default|GetEnemy_Array) OtherActor)
  (if (not (Variables|Default|GetTarget%20Found))
    (CallFunction|FindTarget)))

(event OnComponentEndOverlap(Range)
  (params (OtherActor :type Actor%20Object%20Reference) (OtherComp :type Primitive%20Component%20Object%20Reference) (OtherBodyIndex :type Integer))
  (if (== (Variables|Default|GetEnemy_Ref) OtherActor)
    (CallFunction|FindTarget))
  (Utilities|Array|RemoveItem (Variables|Default|GetEnemy_Array) OtherActor))

(event EventTick
  (params (DeltaSeconds :type Float%20%28single-precision%29))
  (if (Variables|Default|GetTarget%20Found)
    (bind _inrange (CallFunction|CheckRange (Variables|Default|GetEnemy_Ref)))
    (if _inrange
      (Math|Float|CompareFloat (Variables|Default|GetFire%20CD) (Utilities|Time|GetGameTimeinSeconds)
        (:>
          (if (and (Variables|Default|GetIsFiring) (Variables|Default|GetTarget%20Found))
            (CallFunction|SetParticleParameters (Variables|Default|GetEnemy_Ref))))
        (:<
          (CallFunction|DealDamage (Variables|Default|GetEnemy_Ref))
          (Variables|Default|SetFire%20CD (+ (Utilities|Time|GetGameTimeinSeconds) (Variables|Default|Get1AttackEveryXSeconds)))
          (CallFunction|FireBeam)
          (Variables|Default|SetIsFiring true)))
      (else
        (CallFunction|FindTarget :!label _label)))
    (else
      (goto _label))))

(event EventBeginPlay
  (Components|Sphere|SetSphereRadius (Variables|Default|GetRange) (Variables|Default|GetRange_Ref) true)
  (Input|EnableInput (Game|GetPlayerController 0)))

(event Input|KeyboardEvents|R
  (:Pressed
    (Components|MoveComponentTo (Variables|Default|GetDefaultSceneRoot) "100.000000,100.000000, 0" "0, 0, 0" false true 1.0)))

(event Input|KeyboardEvents|F
  (:Pressed
    (Components|MoveComponentTo (Variables|Default|GetDefaultSceneRoot) "800.000000,800.000000, 0" "0, 0, 0" false false 0.2)))

(fn ConstructionScript)

(fn FindTarget
  (bind _array_element (Utilities|Array|ForEachLoopwithBreak (Variables|Default|GetEnemy_Array) :!label _label)
    (:LoopBody
      (if (Utilities|IsValid _array_element)
        (bind _asenemy_bp (Utilities|Casting|CastToEnemy_BP _array_element))
        (if (or (or (and (> (Variables|/Script/MyProject18.Enemy|GetRed_Health _asenemy_bp) 0.0) (> (Variables|Default|GetRed_Damage) 0.0)) (and (> (Variables|/Script/MyProject18.Enemy|GetBlue_Health _asenemy_bp) 0.0) (> (Variables|Default|GetBlue_Damage) 0.0))) (and (> (Variables|/Script/MyProject18.Enemy|GetGreen_Health _asenemy_bp) 0.0) (> (Variables|Default|GetGreen_Damage) 0.0)))
          (Variables|Default|SetEnemy_Ref _asenemy_bp)
          (goto _label Break))))
    (:Completed
      (Variables|Default|SetTarget%20Found true)
      (return (Variables|Default|GetEnemy_Ref)))))

(fn DealDamage
  (params (Target :type Enemy%20Object%20Reference))
  (bind _enemy_ref (Variables|Default|GetEnemy_Ref))
  (Variables|Default|SetIsFiring true)
  (if (Variables|Default|GetTarget%20Found)
    (if (Utilities|IsValid Target)
      (bind _isvalid (CallFunction|IsTargetValid Target))
      (if _isvalid
        (Game|Damage|ApplyDamage _enemy_ref (Variables|Default|GetRed_Damage) 0 0 "/Game/Enemy/DamageTypes/RedDamage.RedDamage_C")
        (Game|Damage|ApplyDamage _enemy_ref (Variables|Default|GetBlue_Damage) 0 0 "/Game/Enemy/DamageTypes/BlueDamage.BlueDamage_C")
        (Game|Damage|ApplyDamage _enemy_ref (Variables|Default|GetGreen_Damage) 0 0 "/Game/Enemy/DamageTypes/GreenDamage.GreenDamage_C")
        (else
          (Utilities|Array|RemoveItem (Variables|Default|GetEnemy_Array) Target)
          (Variables|Default|SetTarget%20Found false)))
      (else
        (Variables|Default|SetTarget%20Found false)))))

(fn CheckRange
  (params (EnemyToCheck :type Enemy%20BP%20Object%20Reference))
  (if (Utilities|IsValid EnemyToCheck)
    (if (<= (Transformation|GetDistanceTo EnemyToCheck self) (Variables|Default|GetRange_Ref))
      (Variables|Default|SetInRange true)
      (else
        (Variables|Default|SetInRange false :!label _label)))
    (else
      (goto _label)))
  (return (Variables|Default|GetInRange)))

(fn FireProjectile
  (params (Target :type Enemy%20Object%20Reference))
  (bind _returnvalue (Game|SpawnActorfromClass "/Game/Projectile/Projectile_BP.Projectile_BP_C" (Transformation|GetActorTransform Target) false 0 0))
  (Variables|/Script/Engine.ProjectileMovementComponent|SetHomingTargetComponent (Variables|/Game/Projectile/Projectile_BP.Projectile_BP_C|GetProjectileMovement _returnvalue) (Variables|Default|GetSphere))
  (Rendering|Material|SetScalarParameterValue (Variables|/Game/Projectile/Projectile_BP.Projectile_BP_C|GetDynamicMatinst _returnvalue) "Red Damage" (/ (Variables|Default|GetRed_Damage) 1e+03) :!class /Script/Engine.MaterialInstanceDynamic)
  (Rendering|Material|SetScalarParameterValue (Variables|/Game/Projectile/Projectile_BP.Projectile_BP_C|GetDynamicMatinst _returnvalue) "Blue Damage" (/ (Variables|Default|GetBlue_Damage) 1e+03) :!class /Script/Engine.MaterialInstanceDynamic)
  (Rendering|Material|SetScalarParameterValue (Variables|/Game/Projectile/Projectile_BP.Projectile_BP_C|GetDynamicMatinst _returnvalue) "Green Damage" (/ (Variables|Default|GetGreen_Damage) 1e+03) :!class /Script/Engine.MaterialInstanceDynamic))

(fn IsTargetValid
  (params (Target :type Enemy%20Object%20Reference))
  (bind _asenemy_bp (Utilities|Casting|CastToEnemy_BP Target)
    (:then
      (if (Math|Boolean|ORBoolean (and (> (Variables|/Script/MyProject18.Enemy|GetRed_Health _asenemy_bp) 0.0) (> (Variables|Default|GetRed_Damage) 0.0)) (and (> (Variables|/Script/MyProject18.Enemy|GetBlue_Health _asenemy_bp) 0.0) (> (Variables|Default|GetBlue_Damage) 0.0)) (and (> (Variables|/Script/MyProject18.Enemy|GetGreen_Health _asenemy_bp) 0.0) (> (Variables|Default|GetGreen_Damage) 0.0)))
        (Variables|Default|SetisValidTarget true)
        (else
          (Variables|Default|SetisValidTarget false))))
    (:CastFailed
      (Development|PrintString "Enemy Validation Cast Failed")))
  (return (Variables|Default|GetisValidTarget)))

(fn SetParticleParameters
  (params (target :type Enemy%20Object%20Reference))
  (bind _returnvalue (Transformation|GetActorLocation target))
  (bind _particlelightning (Variables|Default|GetParticleLightning))
  (Class|ParticleSystemComponent|SetBeamTargetPoint _particlelightning 0 _returnvalue)
  (Class|ParticleSystemComponent|SetBeamTargetPoint _particlelightning 1 _returnvalue))

(fn FireBeam
  (bind _blue_damage (Variables|Default|GetBlue_Damage))
  (bind _red_damage (Variables|Default|GetRed_Damage))
  (bind _green_damage (Variables|Default|GetGreen_Damage))
  (bind _returnvalue (/ _red_damage 1e+03))
  (bind _returnvalue_2 (/ _blue_damage 1e+03))
  (bind _returnvalue_3 (/ _green_damage 1e+03))
  (bind _returnvalue_4 (Math|Vector|MakeVector _returnvalue _returnvalue_3 _returnvalue_2))
  (if (Variables|Default|GetTarget%20Found)
    (if (Variables|Default|GetIsFiring)
      (bind _returnvalue_5 (Effects|SpawnEmitteratLocation "/Game/ScifiParticlePack/Particles/P_BeamLightning.P_BeamLightning" (Transformation|GetWorldLocation (Variables|Default|GetSphere))))
      (Variables|Default|SetParticleLightning _returnvalue_5)
      (Effects|Components|ParticleSystem|SetVectorParameter _returnvalue_5 "Arc_Color" _returnvalue_4)
      (Effects|Components|ParticleSystem|SetVectorParameter _returnvalue_5 "Arc_Color1" _returnvalue_4))))